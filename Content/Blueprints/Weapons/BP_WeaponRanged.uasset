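; Ranged weapon Blueprint that handles the HUD and impact responses to reload and firing events.
; Reload and bullet-fired events share one path that tells player 0's BP_HUD to update ammo.
; Hitscan hits spawn a small explosion emitter, marked as a test placeholder for Niagara.
; If the hit actor's root simulates physics, the hit component gets an impulse along the muzzle socket's forward direction.
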(event `self.BP_OnReload`
  (bind _returnvalue (`GameplayStatics.GetPlayerController` 0))
  (bind _returnvalue_2 (`PlayerController.GetHUD` _returnvalue))
  (`/Engine/EditorBlueprintResources/StandardMacros.IsValid` _returnvalue :!label _label
    (:`Is Valid`
      (`/Engine/EditorBlueprintResources/StandardMacros.IsValid` _returnvalue_2
        (:`Is Valid`
          (bind _asbp_hud (cast `/Game/Blueprints/UI/BP_HUD` _returnvalue_2))
          (`/Engine/EditorBlueprintResources/StandardMacros.IsValid` _asbp_hud
            (:`Is Valid`
              (`/Game/Blueprints/UI/BP_HUD.OnAmmoUpdated` _asbp_hud))))))))

(event `self.BP_OnBulletFired`
  (goto _label))

(event `self.BP_OnHitScanBulletFired`
  (params (HitResultLocation :type "Vector Structure") (HitActor :type "Actor Object Reference") (HitComponent :type "PrimitiveComponent Object Reference"))
  (bind (_returnvalue_location _returnvalue_rotation) (`KismetMathLibrary.BreakTransform` (`SceneComponent.GetSocketTransform` (`self.WeaponSkeletalMesh`) "Muzzle" "RTS_World")))
  ;[1 1 1] Move to Niagara System (purely for testing)
  (`GameplayStatics.SpawnEmitterAtLocation` "/Game/StarterContent/Particles/P_Explosion.P_Explosion" HitResultLocation (struct) (0.3 0.3 0.3))
  (if (`SceneComponent.IsSimulatingPhysics` (`Actor.RootComponent` HitActor) "None")
    (`PrimitiveComponent.AddImpulseAtLocation` HitComponent (* (`KismetMathLibrary.GetForwardVector` _returnvalue_rotation) 20000.0) HitResultLocation "None")))

(fn `UserConstructionScript`)